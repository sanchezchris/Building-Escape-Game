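; Door actor that swings open in either of two directions and closes again.
; It caches its starting rotation on BeginPlay and responds to normal-open, reverse-open and two close events from OpenDoor.
; Two timelines, DoorSwing and DoorSwingReversed, drive a yaw offset combined with that starting rotation.
; Each close event plays its matching timeline in reverse.
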(event OnOpenNormal(OpenDoor)
  (bind _open_angletrack (Timeline|Door%20Swing Play)
    (:Update
      (Transformation|SetActorRotation (Math|Rotator|CombineRotators (Math|Rotator|MakeRotator 0.0 0.0 _open_angletrack) (Variables|Default|GetInitial%20Rotation))))))

(event OnOpenReverse(OpenDoor)
  (bind _open_angletrack (Timeline|Door%20Swing%20Reversed Play)
    (:Update
      (Transformation|SetActorRotation (Math|Rotator|CombineRotators (Math|Rotator|MakeRotator 0.0 0.0 _open_angletrack) (Variables|Default|GetInitial%20Rotation))))))

(event OnClose1(OpenDoor)
  (bind _open_angletrack (Timeline|Door%20Swing Reverse)
    (:Update
      (Transformation|SetActorRotation (Math|Rotator|CombineRotators (Math|Rotator|MakeRotator 0.0 0.0 _open_angletrack) (Variables|Default|GetInitial%20Rotation))))))

(event OnClose2(OpenDoor)
  (bind _open_angletrack (Timeline|Door%20Swing%20Reversed Reverse)
    (:Update
      (Transformation|SetActorRotation (Math|Rotator|CombineRotators (Math|Rotator|MakeRotator 0.0 0.0 _open_angletrack) (Variables|Default|GetInitial%20Rotation))))))

(event EventBeginPlay
  (Variables|Default|SetInitial%20Rotation (Transformation|GetActorRotation)))

(fn ConstructionScript)